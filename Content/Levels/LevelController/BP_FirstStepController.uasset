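; BP_FirstStepController is a level trigger that hides the "Floor2" level geometry while the top-down character overlaps it.
; On begin overlap, it finds all actors tagged "Floor2", hides them and disables their collision.
; On end overlap, it repeats the tag lookup and restores their visibility and collision.
; Both events respond only to BP_TopDownCharacter.
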(event `self.ReceiveActorBeginOverlap`
  (params (OtherActor :type "Actor Object Reference"))
  (cast `/Game/TopDown/Blueprints/BP_TopDownCharacter` OtherActor)
  (bind _outactors (`GameplayStatics.GetAllActorsWithTag` "Floor2"))
  (for _array_element _outactors
    (`self.SetActorHiddenInGame` _array_element true :!label _label)
    (`self.SetActorEnableCollision` _array_element false))
  (goto _label))

(event `self.ReceiveActorEndOverlap`
  (params (OtherActor :type "Actor Object Reference"))
  (cast `/Game/TopDown/Blueprints/BP_TopDownCharacter` OtherActor)
  (bind _outactors (`GameplayStatics.GetAllActorsWithTag` "Floor2"))
  (for _array_element _outactors
    (`self.SetActorHiddenInGame` _array_element false :!label _label_2)
    (`self.SetActorEnableCollision` _array_element true))
  (goto _label_2))

(fn `UserConstructionScript`)